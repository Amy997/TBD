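; BP_firelight is a Blueprint with a point light, apparently intended as an animated firelight.
; On BeginPlay it sets the light intensity from Brightness1, then raises that variable by one step if below a cap, without reapplying it.
; The retriggerable delay loop that would repeat the ramp and the random red-to-yellow color change are both disconnected, so the light stays static.
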(event EventBeginPlay
  (Rendering|Components|Light|SetIntensity (Variables|Default|GetPointLight) (Variables|Default|Getbrightness1))
  (if (not (>= (Variables|Default|Getbrightness1) 2e+03))
    (Variables|Default|Setbrightness1 (+ (Variables|Default|Getbrightness1) 1e+01))))

(event Collision|EventActorBeginOverlap
  (params (OtherActor :type Actor%20Object%20Reference)))

(event EventTick
  (params (DeltaSeconds :type Float%20%28single-precision%29)))

(fn ConstructionScript)